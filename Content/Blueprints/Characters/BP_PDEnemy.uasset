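; BP_PDEnemy is an enemy character that chases the player and deals contact damage.
; PawnSensing sightings set IsSeeingPlayer, never cleared here, and call FollowPawn, which issues an AI MoveTo toward the first player character regardless of which pawn was seen.
; Capsule hits apply fixed damage when the other actor matches the AsBPPDCharacterPawn reference, which this graph never assigns.
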(event `self.PawnSensing.OnSeePawn`
  (params (Pawn :type "Pawn Object Reference"))
  (set `self.IsSeeingPlayer` true)
  (`self.FollowPawn`))

(event `FollowPawn`
  (if (`self.IsSeeingPlayer`)
    (`|AIMoveTo` self (0.0 0.0 0.0) (`GameplayStatics.GetPlayerCharacter` 0))))

(event `self.CapsuleComponent.OnComponentHit`
  (params (HitComponent :type "PrimitiveComponent Object Reference") (OtherActor :type "Actor Object Reference") (OtherComp :type "PrimitiveComponent Object Reference") (NormalImpulse :type "Vector Structure") (Hit :type "HitResult Structure (by ref)"))
  (bind _as_bp_pdcharacter_pawn (`self.As BP PDCharacter Pawn`))
  (if (== OtherActor _as_bp_pdcharacter_pawn)
    (`GameplayStatics.ApplyDamage` _as_bp_pdcharacter_pawn 2.0 null self)))

(fn `UserConstructionScript`)